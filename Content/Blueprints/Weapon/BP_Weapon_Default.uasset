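; BP_Weapon_Default is a car-mounted weapon that fires a pair of projectiles from the instigating BP_MyCar.
; UseWeapon calls the parent implementation and runs SpawnProjectile only when that returns true.
; SpawnProjectile casts the instigator to the car and spawns ProjectileClass slightly ahead of its RightShooter and LeftShooter, matching their rotation.
; Each projectile receives the weapon's Damage, with the weapon as owner and the same instigator.
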(fn `SpawnProjectile`
  (bind _asbp_my_car (cast `/Game/Blueprints/Player/BP_MyCar` (`self.GetInstigator`)))
  (`|ExecutionSequence`
    (:`then_0`
      (bind _rightshooter (`/Game/Blueprints/Player/BP_MyCar.RightShooter` _asbp_my_car))
      (`|SpawnActorFromClass` (`self.ProjectileClass`) (`KismetMathLibrary.MakeTransform` (+ (`SceneComponent.K2_GetComponentLocation` _rightshooter) (* (`SceneComponent.GetForwardVector` _rightshooter) 70)) (`SceneComponent.K2_GetComponentRotation` _rightshooter)) "Undefined" "OverrideRootScale" self (`self.Damage`) (`self.GetInstigator`)))
    (:`then_1`
      (bind _leftshooter (`/Game/Blueprints/Player/BP_MyCar.LeftShooter` _asbp_my_car))
      (`|SpawnActorFromClass` (`self.ProjectileClass`) (`KismetMathLibrary.MakeTransform` (+ (`SceneComponent.K2_GetComponentLocation` _leftshooter) (* (`SceneComponent.GetForwardVector` _leftshooter) 70)) (`SceneComponent.K2_GetComponentRotation` _leftshooter)) "Undefined" "OverrideRootScale" self (`self.Damage`) (`self.GetInstigator`)))))

(fn `UserConstructionScript`
  (`parent.UserConstructionScript`))

(fn `UseWeapon`
  (params (Use :type Boolean))
  (returns (Used :type Boolean))
  (bind _used (`parent.UseWeapon` Use))
  (if _used
    (`self.SpawnProjectile`)))