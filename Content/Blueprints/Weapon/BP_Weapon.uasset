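; BP_Weapon is a weapon Blueprint that handles use and cooldown, with no firing effects of its own.
; UseWeapon checks that no cooldown timer is active, then flags the weapon as in use, starts the timer and calls WeaponUsed.
; When the cooldown ends, ShootDelay clears the timer and calls UseWeapon again, so use repeats automatically; passing false does not stop it.
; UsingWeapon has an empty OnRep handler.
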(fn `AbleToUseWeapon`
  (returns (Use :type Boolean))
  (return (not (`KismetSystemLibrary.K2_IsValidTimerHandle` (`self.CooldownTimer`)))))

(fn `OnRep_UsingWeapon`)

(fn `ShootDelay`
  (`KismetSystemLibrary.K2_ClearAndInvalidateTimerHandle` (`self.CooldownTimer`))
  (`self.UseWeapon` true))

(fn `UserConstructionScript`)

(fn `UseWeapon`
  (params (Use :type Boolean))
  (returns (Used :type Boolean))
  (if Use
    (if (`self.AbleToUseWeapon`)
      (set `self.UsingWeapon` true)
      (bind _returnvalue (`KismetSystemLibrary.K2_SetTimer` null "ShootDelay" (`self.CooldownTime`)))
      (set `self.CooldownTimer` _returnvalue)
      (`self.WeaponUsed`)
      (return true)
      (else
        (set `self.UsingWeapon` false)))))