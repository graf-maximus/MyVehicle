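; BP_HealthComponent is an actor component that tracks health for a BP_MyCar owner and destroys the car when health runs out.
; At BeginPlay it sets health to maximum, caches the owning car and, on the server only, binds to the car's point-damage event.
; Each hit subtracts damage through ApplyDamage, which reports whether health reached zero so the handler can destroy the car.
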(event `self.ReceiveBeginPlay`
  (set `self.CurrentHealth` (`self.MaxHealth`))
  (bind _asbp_my_car (cast `/Game/Blueprints/Player/BP_MyCar` (`self.GetOwner`)))
  (bind _output_get (set `self.Car` _asbp_my_car))
  (if (`KismetSystemLibrary.IsServer`)
    (add `Actor.OnTakePointDamage` _output_get (delegate `OnCarTakePointDamage`))))

(event `OnCarTakePointDamage`
  (params (DamagedActor :type "Actor Object Reference") (Damage :type "Float (double-precision)") (InstigatedBy :type "Controller Object Reference") (HitLocation :type "Vector Structure") (FHitComponent :type "PrimitiveComponent Object Reference") (BoneName :type Name) (ShotFromDirection :type "Vector Structure") (DamageType :type "DamageType Object Reference") (DamageCauser :type "Actor Object Reference"))
  (bind _isdead_ (`self.ApplyDamage` Damage))
  (if _isdead_
    (`Actor.K2_DestroyActor` (`self.Car`))))

(fn `ApplyDamage`
  (params (Damage :type "Float (double-precision)"))
  (returns (`IsDead?` :type Boolean))
  (bind _output_get (set `self.CurrentHealth` (- (`self.CurrentHealth`) Damage)))
  (return (<= _output_get 0.0)))