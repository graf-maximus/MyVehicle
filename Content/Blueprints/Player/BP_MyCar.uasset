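; Player car pawn that drives, fires a mounted weapon and takes projectile damage.
; Input axes feed throttle and steering to VehicleMovement and rotate the SpringArm, yaw in world space and pitch in local space.
; Fire press and release toggle the weapon component's main weapon.
; Mesh overlaps with BP_Projectile pass its damage to the health component, destroying the car when ApplyDamage returns true.
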(event `InputAxis|Forward`
  (params (AxisValue :type "Float (single-precision)"))
  (`WheeledVehicleMovementComponent.SetThrottleInput` (`self.VehicleMovement`) AxisValue))

(event `InputAxis|Right`
  (params (AxisValue :type "Float (single-precision)"))
  (`WheeledVehicleMovementComponent.SetSteeringInput` (`self.VehicleMovement`) AxisValue))

(event `InputAxis|YawInput`
  (params (AxisValue :type "Float (single-precision)"))
  (`SceneComponent.K2_AddWorldRotation` (`self.SpringArm`) (`KismetMathLibrary.MakeRotator` 0.0 0.0 AxisValue) false false))

(event `InputAxis|RollInput`
  (params (AxisValue :type "Float (single-precision)"))
  (`SceneComponent.K2_AddLocalRotation` (`self.SpringArm`) (`KismetMathLibrary.MakeRotator` 0.0 AxisValue) false false))

(event `InputAction|Fire`
  (params (Key :type "Key Structure"))
  (:`Pressed`
    (bind _bp_weaponcomponent (`self.BP_WeaponComponent`)
      (:`then`
        (bind _mainweapon (`/Game/Blueprints/Components/BP_WeaponComponent.MainWeapon` _bp_weaponcomponent)
          (:`then`
            (`/Game/Blueprints/Weapon/BP_Weapon.UseWeapon` _mainweapon true))
          (:`else`)))
      (:`else`)))
  (:`Released`
    (bind _bp_weaponcomponent_2 (`self.BP_WeaponComponent`)
      (:`then`
        (bind _mainweapon_2 (`/Game/Blueprints/Components/BP_WeaponComponent.MainWeapon` _bp_weaponcomponent_2)
          (:`then`
            (`/Game/Blueprints/Weapon/BP_Weapon.UseWeapon` _mainweapon_2 false))
          (:`else`)))
      (:`else`))))

(event `self.Mesh.OnComponentBeginOverlap`
  (params (OverlappedComponent :type "PrimitiveComponent Object Reference") (OtherActor :type "Actor Object Reference") (OtherComp :type "PrimitiveComponent Object Reference") (OtherBodyIndex :type Integer) (bFromSweep :type Boolean) (SweepResult :type "HitResult Structure (by ref)"))
  (bind _asbp_projectile (cast `/Game/Blueprints/Weapon/Projectile/BP_Projectile` OtherActor))
  (bind _isdead_ (`/Game/Blueprints/Components/BP_HealthComponent.ApplyDamage` (`self.BP_HealthComponent`) (`/Game/Blueprints/Weapon/Projectile/BP_Projectile.Damage` _asbp_projectile)))
  (if _isdead_
    (`self.K2_DestroyActor`)))

(fn `UserConstructionScript`)