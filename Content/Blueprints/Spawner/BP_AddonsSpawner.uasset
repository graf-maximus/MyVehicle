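; BP_AddonsSpawner spawns a random rocket, mine or invisibility addon pickup on BeginPlay and then periodically.
; SpawnAddon picks the class from the addon enum and places it at random X/Y within the Box extent, centred on world origin, at the Box's height.
; It then fires AddonSpawned, whose handler sets the looping timer for further random spawns.
; Tick prints elapsed spawn and respawn timer values for debugging.
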(event `self.ReceiveBeginPlay`
  (add `self.AddonSpawned` (delegate `OnAddonSpawned`))
  (bind _output_get (set `self.Addons` (cast `/Game/Blueprints/Data/E_Addons` (`KismetMathLibrary.Conv_IntToByte` (`KismetMathLibrary.RandomIntegerInRange` 0 2)))))
  (`self.SpawnAddon` _output_get))

(event `OnAddonSpawned`
  (bind _returnvalue (`KismetSystemLibrary.K2_SetTimerDelegate` (delegate `CustomEvent_0`) 5.0 true))
  (set `self.DefaultSpawnTimer` _returnvalue))

(event `CustomEvent_0`
  (bind _output_get (set `self.Addons` (cast `/Game/Blueprints/Data/E_Addons` (`KismetMathLibrary.Conv_IntToByte` (`KismetMathLibrary.RandomIntegerInRange` 0 3)))))
  (`self.SpawnAddon` _output_get))

(event `self.ReceiveTick`
  (params (DeltaSeconds :type "Float (single-precision)"))
  (`KismetSystemLibrary.PrintString` (`KismetStringLibrary.Conv_DoubleToString` (`KismetSystemLibrary.K2_GetTimerElapsedTimeHandle` (`self.DefaultSpawnTimer`))) true true (struct :`G` 0.66 :`B` 1.0 :`A` 1.0) 0.0)
  (`KismetSystemLibrary.PrintString` (`KismetStringLibrary.Conv_DoubleToString` (`KismetSystemLibrary.K2_GetTimerElapsedTimeHandle` (`self.RespawnTimer`))) true true (struct :`G` 0.66 :`B` 1.0 :`A` 1.0) 0.0))

(fn `SpawnAddon`
  (params (Addon :type "/Game/Blueprints/Data/E_Addons Enum" :default "NewEnumerator0"))
  (bind _box (`self.Box`))
  (bind (_returnvalue_x _returnvalue_y _returnvalue_z) (`KismetMathLibrary.BreakVector` (`SceneComponent.K2_GetComponentLocation` _box)))
  (bind (_returnvalue_x_2 _returnvalue_y_2) (`KismetMathLibrary.BreakVector` (`BoxComponent.GetScaledBoxExtent` _box)))
  (switch `/Game/Blueprints/Data/E_Addons` Addon
    (:`NewEnumerator0`
      (set `self.SpawnedAddonClass` "/Game/Blueprints/Spawner/Spawners/BP_Addon_Rockets.BP_Addon_Rockets_C"))
    (:`NewEnumerator1`
      (set `self.SpawnedAddonClass` "/Game/Blueprints/Spawner/Spawners/BP_Addon_Mine.BP_Addon_Mine_C"))
    (:`NewEnumerator2`
      (set `self.SpawnedAddonClass` "/Game/Blueprints/Spawner/Spawners/BP_Addon_Invise.BP_Addon_Invise_C")))
  (bind _returnvalue (`|SpawnActorFromClass` (`self.SpawnedAddonClass`) (`KismetMathLibrary.MakeTransform` (`KismetMathLibrary.MakeVector` (`KismetMathLibrary.RandomFloatInRange` (* -1 _returnvalue_x_2) _returnvalue_x_2) (`KismetMathLibrary.RandomFloatInRange` (* -1 _returnvalue_y_2) _returnvalue_y_2) _returnvalue_z)) "Undefined" "OverrideRootScale" null null))
  (set `self.SpawnedActor` _returnvalue)
  (`self.AddonSpawned`))

(fn `UserConstructionScript`)